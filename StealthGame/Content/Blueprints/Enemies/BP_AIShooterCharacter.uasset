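; AI shooter enemy character with a health bar widget component that responds to player proximity.
; Each tick it activates or deactivates the Healthbar component based on whether the first player's pawn is within HealthShowRange.
; It also copies GetHealthPercent into the WBP_EnemyHealthBar widget every tick, regardless of distance.
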(event `self.ReceiveBeginPlay`)

(event `self.ReceiveTick`
  (params (DeltaSeconds :type "Float (single-precision)"))
  (`self.ShouldShowWidget`)
  (`self.UpdateHealthBar`))

(fn `ShouldShowWidget`
  (bind _healthbar (`self.Healthbar`))
  (if (<= (`KismetMathLibrary.Vector_Distance` (`self.K2_GetActorLocation`) (`self.K2_GetActorLocation` (`GameplayStatics.GetPlayerPawn` 0))) (`self.HealthShowRange`))
    (`ActorComponent.Activate` _healthbar false)
    (else
      (`ActorComponent.Deactivate` _healthbar)))
  (return))

(fn `UpdateHealthBar`
  (bind _aswbp_enemy_health_bar (cast `/Game/UI/Widgets/WBP_EnemyHealthBar` (`WidgetComponent.GetUserWidgetObject` (`self.Healthbar`))))
  (set `/Game/UI/Widgets/WBP_EnemyHealthBar.Heatlh` (`self.GetHealthPercent`) _aswbp_enemy_health_bar)
  (return))

(fn `UserConstructionScript`)