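; Player character Blueprint that adds surface-dependent footstep audio through its PlayWalkSound function.
; PlayWalkSound line-traces 150 units down from the actor on the Visibility channel and stores the hit physical material as the current surface.
; The hit's surface type selects a wood, grass or tile footstep cue, played at the impact location.
; The event graph and construction script are empty, and nothing here calls the function.
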(fn `PlayWalkSound`
  (bind _returnvalue (`self.K2_GetActorLocation`))
  (bind (_outhit _returnvalue_2) (`KismetSystemLibrary.LineTraceSingle` _returnvalue (- _returnvalue (0.0 0.0 150.0)) "TraceTypeQuery1"))
  (if _returnvalue_2
    (bind (_bblockinghit _binitialoverlap _time _distance _location _impactpoint _normal _impactnormal _physmat) (`GameplayStatics.BreakHitResult` _outhit))
    (`self.SetCurrentSurface` _physmat)
    (switch `EPhysicalSurface` (`GameplayStatics.GetSurfaceType` _outhit)
      (:`SurfaceType1`
        (`GameplayStatics.PlaySoundAtLocation` "/Game/SFX/SoundCues/A_Wood_Footstep_Cue.A_Wood_Footstep_Cue" _location (struct) 1.0 1.0 0.0 null null null null))
      (:`SurfaceType2`
        (`GameplayStatics.PlaySoundAtLocation` "/Game/SFX/SoundCues/A_Grass_Footstep_Cue.A_Grass_Footstep_Cue" _location (struct) 1.0 1.0 0.0 null null null null))
      (:`SurfaceType3`
        (`GameplayStatics.PlaySoundAtLocation` "/Game/SFX/SoundCues/A_Tile_Footstep_Cue.A_Tile_Footstep_Cue" _location (struct) 1.0 1.0 0.0 null null null null)))
    (return)))

(fn `UserConstructionScript`)